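; Boat actor that shuttles back and forth along a straight line from its placed location.
; BeginPlay stores the start location, and Tick lerps to that point plus the EndSpot offset, teleporting without sweep.
; The alpha advances by Speed times delta seconds, and a GoingForward flag reverses it at either end.
; An unconnected sine-based oscillation remains in the graph and never runs.
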(event `self.ReceiveHit`
  (params (MyComp :type "PrimitiveComponent Object Reference") (Other :type "Actor Object Reference") (OtherComp :type "PrimitiveComponent Object Reference") (bSelfMoved :type Boolean) (HitLocation :type "Vector Structure") (HitNormal :type "Vector Structure") (NormalImpulse :type "Vector Structure") (Hit :type "HitResult Structure (by ref)")))

(event `self.ReceiveTick`
  (params (DeltaSeconds :type "Float (single-precision)"))
  (bind _startspot (`self.StartSpot`))
  (bind _returnvalue (* (`self.Speed`) (`GameplayStatics.GetWorldDeltaSeconds`)))
  ;[1 1 1] Lerp
  (`self.K2_SetActorLocation` (`KismetMathLibrary.VLerp` _startspot (+ _startspot (`self.EndSpot`)) (`self.PercentAlongPAth`)) false true)
  (if (`self.GoingForward`)
    (bind _output_get (set `self.PercentAlongPAth` (+ (`self.PercentAlongPAth`) _returnvalue)))
    (if (>= _output_get 1.0)
      (set `self.GoingForward` false))
    (else
      (bind _output_get_2 (set `self.PercentAlongPAth` (- (`self.PercentAlongPAth`) _returnvalue)))
      (if (<= _output_get_2 0.0)
        (set `self.GoingForward` true)))))

(event `self.ReceiveBeginPlay`
  (set `self.StartSpot` (`self.K2_GetActorLocation`)))

(fn `UserConstructionScript`)