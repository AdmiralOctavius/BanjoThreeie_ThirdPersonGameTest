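; Bullet actor Blueprint that awards a point when it hits an Enemy.
; On Hit, it casts the other actor to Enemy, then increments Score on the first player's PlayerController_Banjo.
; It then writes the new score directly into the text of that controller's ScoreWidget.
; The bullet's script neither damages nor destroys the enemy or itself, and BeginPlay, overlap and Tick are unused.
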(event `self.ReceiveHit`
  (params (MyComp :type "PrimitiveComponent Object Reference") (Other :type "Actor Object Reference") (OtherComp :type "PrimitiveComponent Object Reference") (bSelfMoved :type Boolean) (HitLocation :type "Vector Structure") (HitNormal :type "Vector Structure") (NormalImpulse :type "Vector Structure") (Hit :type "HitResult Structure (by ref)"))
  (cast `/Game/Blueprints/Enemy` Other)
  (bind _asplayer_controller_banjo (cast `/Game/Blueprints/PlayerController_Banjo` (`GameplayStatics.GetPlayerController` 0)))
  (bind _output_get (set `/Game/Blueprints/PlayerController_Banjo.Score` (+ (`/Game/Blueprints/PlayerController_Banjo.Score` _asplayer_controller_banjo) 1) _asplayer_controller_banjo))
  (bind _asscore_widget (cast `/Game/UI/ScoreWidget` (`/Game/Blueprints/PlayerController_Banjo.ScoreWidget` _asplayer_controller_banjo)))
  (`TextBlock.SetText` (`/Game/UI/ScoreWidget.ScoreText` _asscore_widget) (`KismetTextLibrary.Conv_IntToText` _output_get)))

(fn `UserConstructionScript`)