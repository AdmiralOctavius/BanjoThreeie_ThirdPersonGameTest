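; Spawner actor that repeatedly spawns instances of a configurable class around its own location.
; BeginPlay starts a timer that calls SpawnActor, which re-arms the same timer after each spawn to form an endless loop.
; Each spawn lands at a random horizontal offset within the radius by flattening a scaled random unit vector to the XY plane, always spawning regardless of collision.
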(event `self.ReceiveTick`
  (params (DeltaSeconds :type "Float (single-precision)")))

(event `self.ReceiveBeginPlay`
  (`KismetSystemLibrary.K2_SetTimer` null "SpawnActor" (`self.Timer`)))

(fn `SpawnActor`
  (bind (_returnvalue_x _returnvalue_y) (`KismetMathLibrary.BreakVector` (* (`KismetMathLibrary.RandomUnitVector`) (`self.Radius`))))
  (`|SpawnActorFromClass` (`self.ClassToReference`) (`KismetMathLibrary.MakeTransform` (+ (`self.K2_GetActorLocation`) (`KismetMathLibrary.MakeVector` _returnvalue_x _returnvalue_y))) "AlwaysSpawn" "OverrideRootScale" null null)
  (`KismetSystemLibrary.K2_SetTimer` null "SpawnActor" (`self.Timer`)))

(fn `UserConstructionScript`)