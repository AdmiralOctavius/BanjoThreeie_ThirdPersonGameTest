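; Crystal actor Blueprint that spawns a TestOBJ at its own location, on a timer or when the player touches it.
; While IsActive is true, Tick spawns once game time passes LastSpawnTime plus SpawnRate.
; Overlap by a playerCharacter feeds the same spawn node directly, bypassing both checks.
; The graph never updates LastSpawnTime, so timed spawning repeats every frame once the threshold passes.
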(event `self.ReceiveTick`
  (params (DeltaSeconds :type "Float (single-precision)"))
  (if (`self.IsActive`)
    (if (>= (`KismetSystemLibrary.GetGameTimeInSeconds`) (+ (`self.lastSpawnTime`) (`self.SpawnRate`)))
      (`|SpawnActorFromClass` "/Game/Blueprints/TestOBJ.TestOBJ_C" (`KismetMathLibrary.MakeTransform` (`self.K2_GetActorLocation`)) "Undefined" "OverrideRootScale" null null :!label _label))))

(event `self.ReceiveActorBeginOverlap`
  (params (OtherActor :type "Actor Object Reference"))
  (cast `/Game/Blueprints/playerCharacter` OtherActor)
  (goto _label))

(fn `UserConstructionScript`)