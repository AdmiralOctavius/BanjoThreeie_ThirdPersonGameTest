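; Drawbridge actor that rotates itself about its roll axis as soon as play begins, with no trigger.
; BeginPlay stores the starting roll, then Tick adds a fixed rotation step to the root component until roll reaches that start plus MinRotation.
; The step ignores delta time, so speed depends on frame rate.
; MaxRotation and a world-rotation node are left unused.
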(event `self.ReceiveBeginPlay`
  (bind _returnvalue_roll (`KismetMathLibrary.BreakRotator` (`self.K2_GetActorRotation`)))
  (set `self.StartRotation` _returnvalue_roll))

(event `self.ReceiveTick`
  (params (DeltaSeconds :type "Float (single-precision)"))
  (if (not (>= (.roll (`self.K2_GetActorRotation`)) (+ (`self.StartRotation`) (`self.MinRotation`))))
    (`SceneComponent.K2_AddRelativeRotation` (`self.DefaultSceneRoot`) (struct :`Roll` 2.0) false false)))

(fn `UserConstructionScript`)